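; BP_L1_Character is the Level 1 player character, handling basic movement, look and jump through Enhanced Input.
; When a player controller takes control, it adds the IMC_Default mapping context to that local player's input subsystem.
; Move actions apply input along the actor's forward and right vectors, look drives controller yaw and pitch scaled by LookSensitivity, and the jump action starts or stops jumping.
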(event `self.ReceiveControllerChanged`
  (params (OldController :type "Controller Object Reference") (NewController :type "Controller Object Reference"))
  (bind _asplayer_controller (cast `PlayerController` NewController))
  (message `EnhancedInputSubsystemInterface.AddMappingContext` (pcsubsystem `EnhancedInputLocalPlayerSubsystem` _asplayer_controller) "/Game/Blueprint/Inputs/IMC_Default.IMC_Default" 0 (struct)))

(event `EnhancedInput|/Game/Blueprint/Inputs/IA_Look`
  (params (ActionValue :type "Vector2D Structure") (ElapsedSeconds :type "Float (double-precision)") (TriggeredSeconds :type "Float (double-precision)") (InputAction :type "InputAction Object Reference" :default "/Game/Blueprint/Inputs/IA_Look.IA_Look"))
  (bind _looksensitivity (`self.LookSensitivity`))
  (:`Triggered`
    (`self.AddControllerYawInput` (* ActionValue_X _looksensitivity))
    (`self.AddControllerPitchInput` (* ActionValue_Y _looksensitivity))))

(event `EnhancedInput|/Game/Blueprint/Inputs/IA_MoveForward`
  (params (ActionValue :type "Float (double-precision)") (ElapsedSeconds :type "Float (double-precision)") (TriggeredSeconds :type "Float (double-precision)") (InputAction :type "InputAction Object Reference" :default "/Game/Blueprint/Inputs/IA_MoveForward.IA_MoveForward"))
  (:`Triggered`
    (`self.AddMovementInput` (`self.GetActorForwardVector`) ActionValue)))

(event `EnhancedInput|/Game/Blueprint/Inputs/IA_MoveRight`
  (params (ActionValue :type "Float (double-precision)") (ElapsedSeconds :type "Float (double-precision)") (TriggeredSeconds :type "Float (double-precision)") (InputAction :type "InputAction Object Reference" :default "/Game/Blueprint/Inputs/IA_MoveRight.IA_MoveRight"))
  (:`Triggered`
    (`self.AddMovementInput` (`self.GetActorRightVector`) ActionValue)))

(event `EnhancedInput|/Game/Blueprint/Inputs/IA_Jump`
  (params (ActionValue :type Boolean) (ElapsedSeconds :type "Float (double-precision)") (TriggeredSeconds :type "Float (double-precision)") (InputAction :type "InputAction Object Reference" :default "/Game/Blueprint/Inputs/IA_Jump.IA_Jump"))
  (:`Triggered`
    (if ActionValue
      (`self.Jump`)
      (else
        (`self.StopJumping`)))))

(fn `UserConstructionScript`)