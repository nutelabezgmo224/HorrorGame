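; Interactable door actor that swings open away from the player and closes on the next interaction.
; On opening, the dot product of the door's forward vector and the player-to-door direction picks which way it swings.
; A timeline lerps the door mesh's relative yaw up to a quarter turn either way, and reverses to close it.
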(event `self.Interact`
  (if (`self.DoorIsClosed`)
    (set `self.DoorIsClosed` false)
    (set `self.DotProduct` (`KismetMathLibrary.Dot_VectorVector` (`KismetMathLibrary.Normal` (- (`self.K2_GetActorLocation` self) (`self.K2_GetActorLocation` (`self.PlayerRef`)))) (`self.GetActorForwardVector` self)))
    (bind (_direction _alpha) (`Timeline|OpenDoor_TL` :!label _label)
      (:`Update`
        (`SceneComponent.K2_SetRelativeRotation` (`self.SM_Door`) (`KismetMathLibrary.MakeRotator` 0.0 0.0 (`KismetMathLibrary.Lerp` 0.0 (select `bool` (>= (`self.DotProduct`) 0.0) :`false` -90.0 :`true` 90.0) _alpha)) false false)))
    (else
      (set `self.DoorIsClosed` true)
      (goto _label :!via `Reverse`))))

(fn `UserConstructionScript`
  (`parent.UserConstructionScript`))