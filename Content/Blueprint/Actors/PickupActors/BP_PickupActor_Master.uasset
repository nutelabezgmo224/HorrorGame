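; Base pickup actor that the player either adds to their inventory or uses immediately, with UseItemImmediately left empty.
; A sphere overlap tracks the character, and Tick line-traces to them to show a yaw-billboarded prompt only when unobstructed.
; The prompt toggles within pickup distance, where actor input is also enabled.
; IA_Action adds the item to BPCInventory, keeping any excess amount, or uses it, destroying the actor once consumed.
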(event `self.ReceiveTick`
  (params (DeltaSeconds :type "Float (single-precision)"))
  (bind _returnvalue (`GameplayStatics.GetPlayerController` 0))
  (bind _playerinsidecollision (`self.PlayerInsideCollision`))
  (bind _promptwidget (`self.PromptWidget`))
  (bind (_returnvalue_x _returnvalue_y _returnvalue_z) (`KismetMathLibrary.BreakVector` (`SceneComponent.K2_GetComponentLocation` (`self.StaticMesh`))))
  (bind (_returnvalue_roll _returnvalue_pitch _returnvalue_yaw) (`KismetMathLibrary.BreakRotator` (`SceneComponent.K2_GetComponentRotation` (`/Game/Blueprint/BP_Character.Camera` _playerinsidecollision))))
  (`/Engine/EditorBlueprintResources/StandardMacros.IsValid` _playerinsidecollision
    (:`Is Valid`
      (`SceneComponent.K2_SetWorldLocation` (`self.PromptWidget`) (`KismetMathLibrary.MakeVector` _returnvalue_x _returnvalue_y (+ _returnvalue_z (`self.WidgetDistance`))) false false)
      (bind (_outhit _returnvalue_2) (`KismetSystemLibrary.LineTraceSingle` (`SceneComponent.K2_GetComponentLocation` (`self.StaticMesh`)) (`self.K2_GetActorLocation` _playerinsidecollision) "TraceTypeQuery1"))
      (bind _returnvalue_3 (not _returnvalue_2))
      (`SceneComponent.SetVisibility` _promptwidget _returnvalue_3 false)
      (if _returnvalue_3
        (`SceneComponent.K2_SetWorldRotation` _promptwidget (`KismetMathLibrary.MakeRotator` 0.0 0.0 (- _returnvalue_yaw 180.0)) false false)
        (bind (_bblockinghit _binitialoverlap _time _distance _location _impactpoint _normal _impactnormal _physmat _hitactor _hitcomponent _hitbonename _bonename _hititem _elementindex _faceindex _tracestart _traceend) (`GameplayStatics.BreakHitResult` _outhit))
        (bind _returnvalue_4 (<= (`KismetMathLibrary.VSize` (- _tracestart _traceend)) (`self.PickUpDistance`)))
        (`/Game/UMG/W_PickUpPrompt.TogglePrompt` (cast `/Game/UMG/W_PickUpPrompt` (`WidgetComponent.GetUserWidgetObject` (`self.PromptWidget`)) :!pure true) _returnvalue_4)
        (if _returnvalue_4
          (`self.EnableInput` _returnvalue)
          (else
            (`self.DisableInput` _returnvalue)))
        (else
          (`self.DisableInput` (`GameplayStatics.GetPlayerController` 0)))))))

(event `self.Sphere.OnComponentEndOverlap`
  (params (OverlappedComponent :type "PrimitiveComponent Object Reference") (OtherActor :type "Actor Object Reference") (OtherComp :type "PrimitiveComponent Object Reference") (OtherBodyIndex :type Integer))
  (cast `/Game/Blueprint/BP_Character` OtherActor)
  (set `self.PlayerInsideCollision` null)
  (`SceneComponent.SetVisibility` (`self.PromptWidget`) false false)
  (`self.DisableInput` (`GameplayStatics.GetPlayerController` 0)))

(event `self.Sphere.OnComponentBeginOverlap`
  (params (OverlappedComponent :type "PrimitiveComponent Object Reference") (OtherActor :type "Actor Object Reference") (OtherComp :type "PrimitiveComponent Object Reference") (OtherBodyIndex :type Integer) (bFromSweep :type Boolean) (SweepResult :type "HitResult Structure (by ref)"))
  (bind _asbp_character (cast `/Game/Blueprint/BP_Character` OtherActor))
  (set `self.PlayerInsideCollision` _asbp_character))

(event `EnhancedInput|/Game/Blueprint/Inputs/IA_Action`
  (params (ActionValue :type Boolean) (ElapsedSeconds :type "Float (double-precision)") (TriggeredSeconds :type "Float (double-precision)") (InputAction :type "InputAction Object Reference" :default "/Game/Blueprint/Inputs/IA_Action.IA_Action"))
  (:`Triggered`
    (if (`self.CanBeAddedToInventory`)
      (`KismetSystemLibrary.PrintString` "123")
      (bind (_success _excessamount) (`/Game/Blueprint/ActorComponents/BPC_Inventory.AddItem` (`/Game/Blueprint/BP_Character.BPC_Inventory` (`self.PlayerInsideCollision`)) (`self.Item`) (`self.Amount`)))
      (if _success
        (if (> _excessamount 0)
          (set `self.Amount` _excessamount)
          (else
            (`self.K2_DestroyActor`))))
      (else
        (`self.UseItemImmediately`)
        (`self.K2_DestroyActor`)))))

(fn `UseItemImmediately`)

(fn `UserConstructionScript`
  (`SceneComponent.K2_SetRelativeLocation` (`self.PromptWidget`) (`KismetMathLibrary.MakeVector` 0.0 0.0 (`KismetMathLibrary.Conv_IntToDouble` (`self.WidgetDistance`))) false false))