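; Actor component that manages the player's slot-based inventory of item classes and amounts.
; AddItem fills partial stacks, then empty slots, looping on overflow and returning any excess.
; Every slot write goes through UpdateInventorySlot, which also refreshes the menu's grid widget.
; Slot count lives on BP_PlayerController, expandable to a cap; using consumes one item, dropping spawns a physics pickup via camera trace, and ExamineItem is an empty stub.
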(event `self.ReceiveBeginPlay`
  (`self.ResizeSlotsToUserInventorySize`)
  (bind _returnvalue (`GameplayStatics.GetActorOfClass` "/Game/Blueprint/Actors/Inventory/BP_Examination.BP_Examination_C"))
  (set `self.BP_ExaminationRef` _returnvalue)
  (bind _asbp_character (cast `/Game/Blueprint/BP_Character` (`GameplayStatics.GetPlayerCharacter` 0)))
  (set `self.BP_PlayerRef` _asbp_character))

(fn `AddItem`
  (params (Item :type "/Game/Blueprint/Actors/Inventory/BP_InventoryItem_Master2 Class Reference") (Amount :type Integer))
  (returns (Success :type Boolean) (ExcessAmount :type Integer))
  (locals (LocalAmount :type Integer) (LocalIndex :type Integer) (LocalAddAmount :type Integer) (TryToAddItem :type Boolean :default true) (AddedAtLeastOnce :type Boolean))
  (bind _addedatleastonce (`local.AddedAtLeastOnce`))
  (bind _item (`local.Item`))
  (set `local.LocalAddAmount` Amount)
  (if (`KismetSystemLibrary.IsValidClass` Item)
    (`KismetSystemLibrary.PrintString` "222")
    (while (`local.TryToAddItem`)
      (bind (_success _index _newamount _excessamount) (`self.FindExistingSlot` _item (`local.LocalAddAmount`) (`.MaxStackAmount_9_A5AEC13643470FD1FA5A84B3540D40EE` (break `/Game/Blueprint/Structs/S_ItemData` (defaults `Object` _item)))))
      (if _success
        (set `local.LocalIndex` _index)
        (set `local.LocalAddAmount` _excessamount)
        (`self.UpdateInventorySlot` (`local.LocalIndex`) (`local.Item`) _newamount)
        (set `local.AddedAtLeastOnce` true)
        (set `local.TryToAddItem` (> _excessamount 0))
        (else
          (`KismetSystemLibrary.PrintString` "No free slots")
          (return _addedatleastonce _excessamount))))
    (return _addedatleastonce 0)))

(fn `CheckForEmptySlot`
  (returns (Success :type Boolean) (Index :type Integer))
  (locals (LocalSuccess :type Boolean) (LocalIndex :type Integer))
  (for (_array_element _array_index) (`self.InventorySlots`)
    (if (not (`KismetSystemLibrary.IsValidClass` (`.Item_8_BE41F8AC4DB03EAF32C67BBB0A5DEAF7` (break `/Game/Blueprint/Structs/S_InventoryItems` _array_element))))
      (set `local.LocalSuccess` true)
      (set `local.LocalIndex` _array_index)
      (break)))
  (return (`local.LocalSuccess`) (`local.LocalIndex`)))

(fn `ClearSlotAtIndex`
  (params (Index :type Integer))
  (`self.UpdateInventorySlot` Index))

(fn `DropItem`
  (params (Index :type Integer))
  (bind _index (`local.Index`))
  (bind (_item _amount) (`self.GetItemDataByIndex` _index))
  (bind (_itemdata_itemname _itemdata_icon _itemdata_description _itemdata_maxstackamount _itemdata_pickupactor) (break `/Game/Blueprint/Structs/S_ItemData` (defaults `Object` _item)))
  (bind _camera (`/Game/Blueprint/BP_Character.Camera` (cast `/Game/Blueprint/BP_Character` (`GameplayStatics.GetPlayerCharacter` 0) :!pure true)))
  (bind _returnvalue (`SceneComponent.K2_GetComponentLocation` _camera))
  (bind _returnvalue_2 (+ _returnvalue (* (`SceneComponent.GetForwardVector` _camera) 200.0)))
  (bind (_outhit _returnvalue_3) (`KismetSystemLibrary.LineTraceSingle` _returnvalue _returnvalue_2 "TraceTypeQuery1"))
  (bind _returnvalue_4 (`|SpawnActorFromClass` _itemdata_pickupactor (`KismetMathLibrary.MakeTransform` (select `bool` _returnvalue_3 :`false` _returnvalue_2 :`true` (`.Location` (`GameplayStatics.BreakHitResult` _outhit)))) "Undefined" "MultiplyWithRoot" null null))
  (set `/Game/Blueprint/Actors/PickupActors/BP_PickupActor_Master.Amount` _amount _returnvalue_4)
  (`self.ClearSlotAtIndex` _index)
  (`PrimitiveComponent.SetSimulatePhysics` (`/Game/Blueprint/Actors/PickupActors/BP_PickupActor_Master.StaticMesh` _returnvalue_4) true))

(fn `ExamineItem`
  (params (Index :type Integer)))

(fn `ExpandSlots`
  (params (AddSlots :type Integer))
  (bind _inventorymaxsize (`self.InventoryMaxSize`))
  (bind _asbp_player_controller (cast `/Game/Blueprint/BP_PlayerController` (`GameplayStatics.GetPlayerController` 0) :!pure true))
  (bind _inventoryslots (`/Game/Blueprint/BP_PlayerController.InventorySlots` _asbp_player_controller))
  (bind _returnvalue (+ _inventoryslots AddSlots))
  (if (!= _inventorymaxsize _inventoryslots)
    (set `/Game/Blueprint/BP_PlayerController.InventorySlots` (select `bool` (< _returnvalue _inventorymaxsize) :`false` _inventorymaxsize :`true` _returnvalue) _asbp_player_controller)
    (`self.ResizeSlotsToUserInventorySize`)
    (`/Game/UMG/Inventory/W_InventoryGrid.RefreshSlotsView` (`/Game/UMG/Inventory/W_InventoryMenu.W_InventoryGrid` (`/Game/Blueprint/BP_Character.InventoryMenu` (`self.BP_PlayerRef`))))))

(fn `FindExistingSlot`
  (params (Item :type "/Game/Blueprint/Actors/Inventory/BP_InventoryItem_Master2 Class Reference") (AddingAmount :type Integer) (MaxStackAmount :type Integer))
  (returns (Success :type Boolean) (Index :type Integer) (NewAmount :type Integer) (ExcessAmount :type Integer))
  (locals (LocalSuccess :type Boolean) (LocalIndex :type Integer) (LocalNewAmount :type Integer) (LocalExcessAmount :type Integer))
  (bind (_success _index) (`self.CheckForEmptySlot`))
  (bind _maxstackamount (`local.MaxStackAmount`))
  (bind _maxstackamount_2 (`local.MaxStackAmount`))
  (bind _addingamount (`local.AddingAmount`))
  (bind _returnvalue (> _addingamount _maxstackamount_2))
  (set `local.LocalNewAmount` AddingAmount)
  (if (> MaxStackAmount 1)
    (for (_array_element _array_index) (`self.InventorySlots`)
      (bind (_item _amount) (break `/Game/Blueprint/Structs/S_InventoryItems` _array_element))
      (if (and (`KismetSystemLibrary.IsValidClass` _item) (== _item (`local.Item`)) (< _amount (`local.MaxStackAmount`)))
        (bind _returnvalue_2 (+ _amount (`local.AddingAmount`)))
        (bind _returnvalue_3 (> _returnvalue_2 _maxstackamount))
        (set `local.LocalNewAmount` (select `bool` _returnvalue_3 :`false` _returnvalue_2 :`true` _maxstackamount))
        (set `local.LocalExcessAmount` (select `bool` _returnvalue_3 :`true` (- _returnvalue_2 _maxstackamount)))
        (set `local.LocalSuccess` true)
        (set `local.LocalIndex` _array_index)
        (break)))
    (if (`local.LocalSuccess`)
      (return true (`local.LocalIndex`) (`local.LocalNewAmount`) (`local.LocalExcessAmount`))
      (else
        _)))
  (return _success _index (select `bool` _success :`true` (select `bool` _returnvalue :`false` _addingamount :`true` _maxstackamount_2)) (select `bool` _success :`false` _addingamount :`true` (select `bool` _returnvalue :`true` (- (`local.AddingAmount`) _maxstackamount_2)))))

(fn `GetItemDataByIndex`
  (params (Index :type Integer))
  (returns (Item :type "/Game/Blueprint/Actors/Inventory/BP_InventoryItem_Master2 Class Reference") (Amount :type Integer))
  (bind (_item _amount) (break `/Game/Blueprint/Structs/S_InventoryItems` (`|GetArrayItem` (`self.InventorySlots`) Index)))
  (return _item _amount))

(fn `ResizeSlotsToUserInventorySize`
  (`KismetArrayLibrary.Array_Resize` (`self.InventorySlots`) (`/Game/Blueprint/BP_PlayerController.InventorySlots` (cast `/Game/Blueprint/BP_PlayerController` (`GameplayStatics.GetPlayerController` 0) :!pure true))))

(fn `SubstractItem`
  (params (Index :type Integer) (AmountToSubstract :type Integer))
  (bind (_item _amount) (`self.GetItemDataByIndex` Index))
  (if (< AmountToSubstract _amount)
    (`self.UpdateInventorySlot` Index _item (- _amount AmountToSubstract))
    (else
      (`self.ClearSlotAtIndex` Index))))

(fn `UpdateInventorySlot`
  (params (Index :type Integer) (Item :type "/Game/Blueprint/Actors/Inventory/BP_InventoryItem_Master2 Class Reference") (Amount :type Integer))
  (`KismetArrayLibrary.Array_Set` (`self.InventorySlots`) Index (make `/Game/Blueprint/Structs/S_InventoryItems` Item Amount))
  (`/Game/UMG/Inventory/W_InventorySlot.UpdateSlot` (`|GetArrayItem` (`/Game/UMG/Inventory/W_InventoryGrid.SlotsArray` (`/Game/UMG/Inventory/W_InventoryMenu.W_InventoryGrid` (`/Game/Blueprint/BP_Character.InventoryMenu` (`self.BP_PlayerRef`)))) Index) (`local.Item`) (`local.Amount`) (`local.Index`)))

(fn `UseItem`
  (params (Index :type Integer))
  (bind _returnvalue (`|GenericCreateObject` (`self.GetItemDataByIndex` Index)))
  (`/Game/Blueprint/Actors/Inventory/BP_InventoryItem_Master2.UseItem` _returnvalue null)
  (`self.SubstractItem` (`local.Index`) 1))