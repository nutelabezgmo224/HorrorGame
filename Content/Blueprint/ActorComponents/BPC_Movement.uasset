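; Player movement component that handles walking, sprinting with stamina and crouching by changing the owning character's max walk speed.
; Initialize stores the character reference, and start/stop events drive the run and crouch states, with crouching cancelling sprint and resizing the BP_Character capsule.
; Looping timers drain stamina while sprinting and moving, force a stop when empty, and refill it after a restore delay.
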(event `StartCrouchEvent`
  (`self.StopRunning`)
  (`self.StartCrouching`)
  (bind _asbp_character (cast `/Game/Blueprint/BP_Character` (`self.PlayerRef`)))
  (`/Game/Blueprint/BP_Character.ShortenPlayerCapsuleHeight` _asbp_character))

(event `StartRunningEvent`
  (`self.Run`))

(event `StopCrouchEvent`
  (`self.StopCrouching`)
  (bind _asbp_character (cast `/Game/Blueprint/BP_Character` (`self.PlayerRef`)))
  (`/Game/Blueprint/BP_Character.LengthenPlayerCapsule` _asbp_character))

(event `StopRunningEvent`
  (`self.StopRunning`))

(fn `Initialize`
  (params (Character :type "Character Object Reference"))
  (bind _output_get (set `self.PlayerRef` Character))
  (set `CharacterMovementComponent.MaxWalkSpeed` (`self.WalkSpeed`) (`Character.CharacterMovement` _output_get))
  (set `self.CurrentStamina` (`self.MaxStamina`)))

(fn `IsUserHasVelocity`
  (returns (HasVelocity :type Boolean))
  (return (> (`KismetMathLibrary.VSize` (`NavMovementComponent.GetVelocityForNavMovement` (`Character.CharacterMovement` (`self.PlayerRef`)))) 0.0)))

(fn `RefreshStamina`
  (bind _maxstamina (`self.MaxStamina`))
  (bind _returnvalue (+ (`self.CurrentStamina`) (`self.StaminaRestoreRate`)))
  (if (< _returnvalue _maxstamina)
    (bind _output_get (set `self.CurrentStamina` _returnvalue))
    (`KismetSystemLibrary.PrintString` (`KismetStringLibrary.Conv_DoubleToString` _output_get))
    (else
      (set `self.CurrentStamina` _maxstamina)
      (`KismetSystemLibrary.K2_ClearTimer` null "RefreshStamina"))))

(fn `Run`
  (if (and (not (`self.bCrouching`)) (> (`self.CurrentStamina`) 0.0) (`self.IsUserHasVelocity`))
    (set `self.bRunning` true)
    (`KismetSystemLibrary.K2_ClearTimer` null "RefreshStamina")
    (`self.SetUserMaxSpeed` (`self.SprintSpeed`))
    (`KismetSystemLibrary.K2_SetTimer` null "SprintTimer" 0.1 true)
    (else
      (`KismetSystemLibrary.PrintString` "No stamina or you stay"))))

(fn `SetUserMaxSpeed`
  (params (`Max Walk Speed` :type "Float (single-precision)"))
  (set `CharacterMovementComponent.MaxWalkSpeed` `Max Walk Speed` (`Character.CharacterMovement` (`self.PlayerRef`))))

(fn `SprintTimer`
  (bind _currentstamina (`self.CurrentStamina`))
  (bind _returnvalue (- _currentstamina (`self.StaminaConsumptionRate`)))
  (if (> _returnvalue 0.0)
    (bind _output_get (set `self.CurrentStamina` (select `bool` (`self.IsUserHasVelocity`) :`false` _currentstamina :`true` _returnvalue)))
    (`KismetSystemLibrary.PrintString` (`KismetStringLibrary.Conv_DoubleToString` _output_get))
    (else
      (set `self.CurrentStamina` 0.0)
      (`self.StopRunning`))))

(fn `StartCrouching`
  (`self.SetUserMaxSpeed` (`self.CrouchSpeed`))
  (set `self.bCrouching` true))

(fn `StopCrouching`
  (`self.SetUserMaxSpeed` (`self.WalkSpeed`))
  (set `self.bCrouching` false))

(fn `StopRunning`
  (if (`self.bRunning`)
    (set `self.bRunning` false)
    (`self.SetUserMaxSpeed` (`self.WalkSpeed`))
    (`KismetSystemLibrary.K2_ClearTimer` null "SprintTimer")
    (`KismetSystemLibrary.K2_SetTimer` null "RefreshStamina" 0.1 true false (`self.StaminaRestoreDelay`))))