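; First-person player character with Enhanced Input for looking, moving, jumping, running, crouching and a toggleable flashlight.
; Run and crouch go through BPCMovement, with timeline events that lerp capsule height between standing and crouched.
; Camera line traces drive grab-and-release and interaction through BPI_Grab and BPI_Interaction.
; BeginPlay initializes movement and the HUD, while Tick swaps walk and run head-bob camera shakes by speed and ground state.
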(event `self.ReceiveBeginPlay`
  (`self.Initialize`))

(event `self.ReceiveControllerChanged`
  (params (OldController :type "Controller Object Reference") (NewController :type "Controller Object Reference"))
  (bind _asplayer_controller (cast `PlayerController` NewController))
  (message `EnhancedInputSubsystemInterface.AddMappingContext` (pcsubsystem `EnhancedInputLocalPlayerSubsystem` _asplayer_controller) "/Game/Blueprint/Inputs/IMC_Default.IMC_Default" 0 (struct)))

(event `self.ReceiveTick`
  (params (DeltaSeconds :type "Float (single-precision)"))
  (`self.HeadBob`))

(event `EnhancedInput|/Game/Blueprint/Inputs/IA_Look`
  (params (ActionValue :type "Vector2D Structure") (ElapsedSeconds :type "Float (double-precision)") (TriggeredSeconds :type "Float (double-precision)") (InputAction :type "InputAction Object Reference" :default "/Game/Blueprint/Inputs/IA_Look.IA_Look"))
  (bind _looksensitivity (`self.LookSensitivity`))
  ; Input actions
  (:`Triggered`
    (`self.AddControllerYawInput` (* ActionValue_X _looksensitivity))
    (`self.AddControllerPitchInput` (* ActionValue_Y _looksensitivity))))

(event `EnhancedInput|/Game/Blueprint/Inputs/IA_LMB`
  (params (ActionValue :type Boolean) (ElapsedSeconds :type "Float (double-precision)") (TriggeredSeconds :type "Float (double-precision)") (InputAction :type "InputAction Object Reference" :default "/Game/Blueprint/Inputs/IA_LMB.IA_LMB"))
  (bind _grabbedactor (`self.GrabbedActor`))
  ; Input actions
  (:`Triggered`
    (if ActionValue
      (bind _hitactor (`self.LineTrace` 300.0))
      (if (and (`KismetSystemLibrary.IsValid` _hitactor) (`KismetSystemLibrary.DoesImplementInterface` _hitactor "/Game/Blueprint/Interfaces/BPI_Grab.BPI_Grab_C"))
        (message `/Game/Blueprint/Interfaces/BPI_Grab.GrabObject` _hitactor)
        (set `self.GrabbedActor` _hitactor))
      (elif (`KismetSystemLibrary.IsValid` _grabbedactor)
        (message `/Game/Blueprint/Interfaces/BPI_Grab.ReleaseObject` _grabbedactor)
        (set `self.GrabbedActor` null)))))

(event `EnhancedInput|/Game/Blueprint/Inputs/IA_MoveForward`
  (params (ActionValue :type "Float (double-precision)") (ElapsedSeconds :type "Float (double-precision)") (TriggeredSeconds :type "Float (double-precision)") (InputAction :type "InputAction Object Reference" :default "/Game/Blueprint/Inputs/IA_MoveForward.IA_MoveForward"))
  ; Input actions
  (:`Triggered`
    (`self.AddMovementInput` (`self.GetActorForwardVector`) ActionValue)))

(event `EnhancedInput|/Game/Blueprint/Inputs/IA_MoveRight`
  (params (ActionValue :type "Float (double-precision)") (ElapsedSeconds :type "Float (double-precision)") (TriggeredSeconds :type "Float (double-precision)") (InputAction :type "InputAction Object Reference" :default "/Game/Blueprint/Inputs/IA_MoveRight.IA_MoveRight"))
  ; Input actions
  (:`Triggered`
    (`self.AddMovementInput` (`self.GetActorRightVector`) ActionValue)))

(event `EnhancedInput|/Game/Blueprint/Inputs/IA_FlashlightToggle`
  (params (ActionValue :type Boolean) (ElapsedSeconds :type "Float (double-precision)") (TriggeredSeconds :type "Float (double-precision)") (InputAction :type "InputAction Object Reference" :default "/Game/Blueprint/Inputs/IA_FlashlightToggle.IA_FlashlightToggle"))
  (bind _spotlight (`self.SpotLight`))
  ; Input actions
  (:`Triggered`
    (`SceneComponent.SetVisibility` _spotlight (not (`SceneComponent.bVisible` _spotlight)) false)))

(event `EnhancedInput|/Game/Blueprint/Inputs/IA_Jump`
  (params (ActionValue :type Boolean) (ElapsedSeconds :type "Float (double-precision)") (TriggeredSeconds :type "Float (double-precision)") (InputAction :type "InputAction Object Reference" :default "/Game/Blueprint/Inputs/IA_Jump.IA_Jump"))
  ; Input actions
  (:`Triggered`
    (if ActionValue
      (`self.Jump`)
      (else
        (`self.StopJumping`)))))

(event `EnhancedInput|/Game/Blueprint/Inputs/IA_Run`
  (params (ActionValue :type Boolean) (ElapsedSeconds :type "Float (double-precision)") (TriggeredSeconds :type "Float (double-precision)") (InputAction :type "InputAction Object Reference" :default "/Game/Blueprint/Inputs/IA_Run.IA_Run"))
  (bind _bpc_movement (`self.BPC_Movement`))
  ; Input actions
  (:`Triggered`
    (if ActionValue
      (`/Game/Blueprint/ActorComponents/BPC_Movement.StartRunningEvent` _bpc_movement)
      (else
        (`/Game/Blueprint/ActorComponents/BPC_Movement.StopRunningEvent` _bpc_movement)))))

(event `EnhancedInput|/Game/Blueprint/Inputs/IA_Action`
  (params (ActionValue :type Boolean) (ElapsedSeconds :type "Float (double-precision)") (TriggeredSeconds :type "Float (double-precision)") (InputAction :type "InputAction Object Reference" :default "/Game/Blueprint/Inputs/IA_Action.IA_Action"))
  ; Input actions
  (:`Triggered`
    (bind _hitactor (`self.LineTrace` 250.0))
    (if (and (`KismetSystemLibrary.IsValid` _hitactor) (`KismetSystemLibrary.DoesImplementInterface` _hitactor "/Game/Blueprint/Interfaces/BPI_Interaction.BPI_Interaction_C"))
      (message `/Game/Blueprint/Interfaces/BPI_Interaction.Interact` _hitactor))))

(event `EnhancedInput|/Game/Blueprint/Inputs/IA_Crouch`
  (params (ActionValue :type Boolean) (ElapsedSeconds :type "Float (double-precision)") (TriggeredSeconds :type "Float (double-precision)") (InputAction :type "InputAction Object Reference" :default "/Game/Blueprint/Inputs/IA_Crouch.IA_Crouch"))
  (bind _bpc_movement (`self.BPC_Movement`))
  ; Input actions
  (:`Triggered`
    (if ActionValue
      (`/Game/Blueprint/ActorComponents/BPC_Movement.StartCrouchEvent` _bpc_movement)
      (else
        (`/Game/Blueprint/ActorComponents/BPC_Movement.StopCrouchEvent` _bpc_movement)))))

(event `ShortenPlayerCapsuleHeight`
  (bind (_direction _alpha) (`Timeline|CapsuleTL` :!label _label)
    (:`Update`
      (`CapsuleComponent.SetCapsuleHalfHeight` (`self.CapsuleComponent`) (`KismetMathLibrary.Lerp` 88.0 (`/Game/Blueprint/ActorComponents/BPC_Movement.CrouchHalfHeight` (`self.BPC_Movement`)) _alpha) true))))

(event `LengthenPlayerCapsule`
  (goto _label :!via `Reverse`))

(fn `GetPlayerVelocity`
  (returns (VelocityValue :type "Float (double-precision)"))
  (return (`KismetMathLibrary.VSize` (`NavMovementComponent.GetVelocityForNavMovement` (`self.CharacterMovement`)))))

(fn `HeadBob`
  (bind _returnvalue (`GameplayStatics.GetPlayerCameraManager` 0))
  (bind _headbobshakeinstance (`self.HeadBobShakeInstance`))
  (bind _returnvalue_2 (not (`NavMovementInterface.IsFalling` (`self.CharacterMovement`))))
  (if (and (> (`self.GetPlayerVelocity`) 0.0) _returnvalue_2)
    (bind _output_get (set `self.Running` (and (>= (`self.GetPlayerVelocity`) (`/Game/Blueprint/ActorComponents/BPC_Movement.SprintSpeed` (`self.BPC_Movement`))) _returnvalue_2)))
    (`/Engine/EditorBlueprintResources/StandardMacros.IsValid` _headbobshakeinstance
      (:`Is Valid`
        (bind _returnvalue_3 (select `bool` _output_get :`false` "/Game/Blueprint/CameraShakes/BP_HeadBob_Walk.BP_HeadBob_Walk_C" :`true` "/Game/Blueprint/CameraShakes/BP_HeadBob_Run1.BP_HeadBob_Run1_C" :!type "CameraShakeBase Class Reference"))
        (if (not (== (`GameplayStatics.GetObjectClass` (`self.HeadBobShakeInstance`)) _returnvalue_3))
          (`PlayerCameraManager.StopCameraShake` _returnvalue (`self.HeadBobShakeInstance`) false)
          (bind _returnvalue_4 (`PlayerCameraManager.StartCameraShake` :`self` _returnvalue :`ShakeClass` _returnvalue_3))
          (set `self.HeadBobShakeInstance` _returnvalue_4)))
      (:`Is Not Valid`
        (bind _returnvalue_5 (`PlayerCameraManager.StartCameraShake` :`self` (`GameplayStatics.GetPlayerCameraManager` 0) :`ShakeClass` _returnvalue_3))
        (set `self.HeadBobShakeInstance` _returnvalue_5)))
    (else
      (`/Engine/EditorBlueprintResources/StandardMacros.IsValid` _headbobshakeinstance
        (:`Is Valid`
          (`PlayerCameraManager.StopCameraShake` (`GameplayStatics.GetPlayerCameraManager` 0) (`self.HeadBobShakeInstance`) false)
          (set `self.HeadBobShakeInstance` null))))))

(fn `Initialize`
  (`|ExecutionSequence`
    (:`then_0`
      (`/Game/Blueprint/ActorComponents/BPC_Movement.Initialize` (`self.BPC_Movement`) self))
    (:`then_1`
      (bind _returnvalue (`|CreateWidget` "/Game/UMG/W_MainHUD.W_MainHUD_C"))
      (bind _output_get (set `self.MainHUDRef` _returnvalue))
      (`UserWidget.AddToViewport` _output_get 0))))

(fn `LineTrace`
  (params (Length :type "Float (double-precision)") (DrawDebugType :type "EDrawDebugTrace Enum" :default "None"))
  (returns (HitActor :type "Actor Object Reference"))
  (bind _camera (`self.Camera`))
  (bind _returnvalue (`SceneComponent.K2_GetComponentLocation` _camera))
  (bind _outhit (`KismetSystemLibrary.LineTraceSingle` :`Start` _returnvalue :`End` (+ (* Length (`SceneComponent.GetForwardVector` _camera)) _returnvalue) :`TraceChannel` "TraceTypeQuery1" :`DrawDebugType` DrawDebugType))
  (return (`.HitActor` (`GameplayStatics.BreakHitResult` _outhit))))

(fn `UserConstructionScript`)